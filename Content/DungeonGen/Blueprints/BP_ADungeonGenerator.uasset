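; Dungeon generator Blueprint that turns a grid of cell data into spawned room actors when OnDungeonGenerated fires.
; Each array index maps to a position on a ten-by-ten layout with fixed spacing.
; Cell flags select a MasterRoom (start), EndRoom, DungeonRoom or Void filler actor for that position.
; The start cell's location is recorded, and a PlayerStart spawns right after the MasterRoom, though the raised-transform node in CreatePlayerSpawnLocation is unconnected.
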(event `self.OnDungeonGenerated`
  (set `self.RoomSpacing` 990)
  (for (_array_element _array_index) (`self.Grid`)
    (bind _spawnlocation (`self.VectorCreator` _array_index _array_index))
    (bind (_bisroom _bisstart _bisend) (break `RoomCell` _array_element))
    (`self.SetMasterRoomLocationVector` _spawnlocation _bisstart)
    (`KismetSystemLibrary.PrintText` (`KismetTextLibrary.Conv_VectorToText` _spawnlocation) false)
    (`KismetSystemLibrary.PrintText` (`KismetTextLibrary.Conv_IntToText` _array_index) false true (struct :`R` 1.0 :`A` 1.0) 10.0)
    (`self.SpawnRooms` _bisroom _bisstart _bisend (`KismetMathLibrary.MakeTransform` _spawnlocation))
    (if (`self.IsMasterRoomLastSpawned`)
      (`|SpawnActorFromClass` "/Script/Engine.PlayerStart" (`KismetMathLibrary.MakeTransform` (`KismetMathLibrary.MakeVector` (.x (`self.MasterRoomLocation`)) (.y (`self.MasterRoomLocation`)) (+ (.z (`self.MasterRoomLocation`)) 200.0))) "AdjustIfPossibleButAlwaysSpawn" "MultiplyWithRoot" null null)
      (else
        (`KismetSystemLibrary.PrintText` "Not MasterRoom" false)))))

(fn `SetMasterRoomLocationVector`
  (params (MasterRoomLocation :type "Vector Structure") (IsStart :type Boolean))
  (if IsStart
    (bind _output_get (set `self.MasterRoomLocation` MasterRoomLocation))
    (`KismetSystemLibrary.PrintText` (`KismetTextLibrary.Conv_VectorToText` _output_get) true true (struct :`R` 1.0 :`B` 0.757919 :`A` 1.0) 10.0)
    (else
      (`KismetSystemLibrary.PrintText` "Not MasterRoom" false true (struct :`R` 1.0 :`B` 0.861746 :`A` 1.0)))))

(fn `SpawnRooms`
  (params (IsRoom :type Boolean) (IsStart :type Boolean) (IsEnd :type Boolean) (SpawnTransform :type "Transform Structure"))
  (if IsRoom
    (if IsStart
      (`|SpawnActorFromClass` "/Game/DungeonGen/Meshes/MasterRoom.MasterRoom_C" SpawnTransform "AdjustIfPossibleButAlwaysSpawn" "MultiplyWithRoot" null null)
      (set `self.IsMasterRoomLastSpawned` true)
      (else
        (if IsEnd
          (`|SpawnActorFromClass` "/Game/DungeonGen/Meshes/EndRoom.EndRoom_C" SpawnTransform "AdjustIfPossibleButAlwaysSpawn" "MultiplyWithRoot" null null)
          (else
            (`|SpawnActorFromClass` "/Game/DungeonGen/Meshes/DungeonRoom.DungeonRoom_C" SpawnTransform "AdjustIfPossibleButAlwaysSpawn" "MultiplyWithRoot" null null)))
        (set `self.IsMasterRoomLastSpawned` false :!label _label)))
    (else
      (`|SpawnActorFromClass` "/Game/DungeonGen/Meshes/Void.Void_C" SpawnTransform "AdjustIfPossibleButAlwaysSpawn" "MultiplyWithRoot" null null)
      (goto _label))))

(fn `UserConstructionScript`)

(fn `VectorCreator`
  (params (X :type Integer) (Y :type Integer))
  (returns (SpawnLocation :type "Vector Structure"))
  (bind _roomspacing (`self.RoomSpacing`))
  (bind _output_get (set `self.X` (mod Y 10)))
  (bind _output_get_2 (set `self.Y` (mod (/ X 10) 10)))
  (bind _output_get_3 (set `self.RoomSpawnLocation` (`KismetMathLibrary.MakeVector` (`KismetMathLibrary.Conv_IntToDouble` (* _roomspacing _output_get)) (`KismetMathLibrary.Conv_IntToDouble` (* _roomspacing _output_get_2)))))
  (return _output_get_3))